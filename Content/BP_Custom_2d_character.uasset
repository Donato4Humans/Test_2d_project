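; BP_Custom_2d_character is a 2D character Blueprint that shows its health on an on-screen HUD.
; On BeginPlay it creates WBP_HUD, stores the reference, adds it to the viewport and pushes current and default values from its Health member.
; On AnyDamage it pushes those values again if the HUD reference is valid.
; It does no damage math itself, and Tick and overlap events are unused.
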(event `self.ReceiveBeginPlay`
  (bind _health (`self.Health`))
  (bind _returnvalue (`|CreateWidget` "/Game/WBP_HUD.WBP_HUD_C"))
  (bind _output_get (set `self.HUD_Ref` _returnvalue))
  (`UserWidget.AddToViewport` _output_get 0)
  (`/Game/WBP_HUD.UpdateHealth` (`self.HUD_Ref`) (`HealthComponent.Health` _health) (`HealthComponent.DefaultHealth` _health)))

(event `self.ReceiveAnyDamage`
  (params (Damage :type "Float (single-precision)") (DamageType :type "DamageType Object Reference") (InstigatedBy :type "Controller Object Reference") (DamageCauser :type "Actor Object Reference"))
  (bind _health (`self.Health`))
  (`/Engine/EditorBlueprintResources/StandardMacros.IsValid` (`self.HUD_Ref`)
    (:`Is Valid`
      (`/Game/WBP_HUD.UpdateHealth` (`self.HUD_Ref`) (`HealthComponent.Health` _health) (`HealthComponent.DefaultHealth` _health)))))

(fn `UserConstructionScript`)